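; Contact bomb projectile preset that overrides how the projectile is cleaned up when destroyed.
; On authority, DestroyProjectile starts a short timer for delayed destruction and multicasts the shutdown of bomb effects.
; The multicast stops physics and audio, hides the mesh, then deactivates the smoke trail and sparks while keeping those components visible.
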(event `self.DestroyProjectile`
  ;[1 1 1] Destroy projectile with delay.
  (`/Engine/EditorBlueprintResources/ActorMacros.Switch Has Authority`
    (:`Authority`
      (`KismetSystemLibrary.K2_SetTimerDelegate` (`|CreateDelegate` :!event `K2_DestroyActor`) 2.0)
      (`self.DisableBombEffects (Multicast)`))))

(event `DisableBombEffects (Multicast)`
  (bind _smoketrailparticle (`self.SmokeTrailParticle`))
  ;[1 1 1] Destroy projectile with delay.
  (`PrimitiveComponent.SetSimulatePhysics` (`self.RootMeshComponent`) false)
  (`SceneComponent.SetVisibility` (`self.ProjectileMesh`) false true)
  (`AudioComponent.Stop` (`self.Audio`))
  (`SceneComponent.SetVisibility` _smoketrailparticle true false)
  (`SceneComponent.SetVisibility` (`self.SparksParticle`) true false)
  (`ActorComponent.Deactivate` _smoketrailparticle)
  (`ActorComponent.Deactivate` (`self.SparksParticle`)))

(fn `UserConstructionScript`
  (`parent.UserConstructionScript`))